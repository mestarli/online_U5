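; BP_Ball is a physics ball the player passes with left mouse and that resets after reaching a goal.
; Any actor overlap enables player input and ending one disables it, while the click applies a velocity-change impulse along the player controller's forward vector at PassSpeed.
; The first Tick records the start location via DoOnce.
; When its Collision component overlaps BP_Goal, the ball destroys itself and spawns a replacement there.
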(event `Key|LeftMouseButton`
  (params (Key :type "Key Structure"))
  ;[1 1 1] Left mouse to pass
  (:`Pressed`
    (`PrimitiveComponent.AddImpulse` (`self.Ball`) (* (`self.GetActorForwardVector` (`GameplayStatics.GetPlayerController` 0)) (`self.PassSpeed`)) "None" true)))

(event `self.ReceiveActorBeginOverlap`
  (params (OtherActor :type "Actor Object Reference"))
  ;[1 1 1] Allow player to input
  (`self.EnableInput` (`GameplayStatics.GetPlayerController` 0)))

(event `self.ReceiveActorEndOverlap`
  (params (OtherActor :type "Actor Object Reference"))
  ;[1 1 1] Allow player to input
  (`self.DisableInput` (`GameplayStatics.GetPlayerController` 0)))

(event `self.ReceiveTick`
  (params (DeltaSeconds :type "Float (single-precision)"))
  ;[0 0 0] Get Ball Start Position
  (`/Engine/EditorBlueprintResources/StandardMacros.DoOnce` false
    (:`Completed`
      (bind _output_get (set `self.StartPosition` (`KismetMathLibrary.Conv_VectorToTransform` (`self.K2_GetActorLocation`))))
      (`KismetSystemLibrary.LogString` (`KismetStringLibrary.Conv_TransformToString` _output_get)))))

(event `self.Collision.OnComponentBeginOverlap`
  (params (OverlappedComponent :type "PrimitiveComponent Object Reference") (OtherActor :type "Actor Object Reference") (OtherComp :type "PrimitiveComponent Object Reference") (OtherBodyIndex :type Integer) (bFromSweep :type Boolean) (SweepResult :type "HitResult Structure (by ref)"))
  ;[0 0 0] Destroy & Spawn Ball
  (cast `/Game/Blueprints/BP_Goal` OtherActor)
  (`self.K2_DestroyActor`)
  (`|SpawnActorFromClass` "BP_Ball_C" (`self.StartPosition`) "Undefined" "OverrideRootScale" null null))

(fn `UserConstructionScript`)