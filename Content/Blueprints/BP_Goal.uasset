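; BP_Goal is a goal actor that returns players to their start positions when a BP_Ball enters its trigger.
; If the goal is tagged Goal_Player0 or Goal_Player2, identical branches teleport every BP_ThirdPersonCharacter to its StartPosition.
; A DoOnce re-arms five seconds later, but it precedes the ball cast, so any non-ball overlap leaves it locked.
; It neither updates a score nor moves the ball.
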(event `self.Goal_Trigger.OnComponentBeginOverlap`
  (params (OverlappedComponent :type "PrimitiveComponent Object Reference") (OtherActor :type "Actor Object Reference") (OtherComp :type "PrimitiveComponent Object Reference") (OtherBodyIndex :type Integer) (bFromSweep :type Boolean) (SweepResult :type "HitResult Structure (by ref)"))
  (`/Engine/EditorBlueprintResources/StandardMacros.DoOnce` false :!label _label
    (:`Completed`
      (bind _asbp_ball (cast `/Game/Blueprints/BP_Ball` OtherActor))
      (if (`self.ActorHasTag` "Goal_Player0")
        (bind _outactors (`GameplayStatics.GetAllActorsOfClass` "/Game/Blueprints/BP_ThirdPersonCharacter.BP_ThirdPersonCharacter_C"))
        (for _array_element _outactors
          (`self.K2_SetActorLocation` _array_element (`/Game/Blueprints/BP_ThirdPersonCharacter.StartPosition` _array_element) false true))
        (`KismetSystemLibrary.Delay` 5.0)
        (goto _label :!via `Reset`)
        (elif (`self.ActorHasTag` "Goal_Player2")
          (bind _outactors_2 (`GameplayStatics.GetAllActorsOfClass` "/Game/Blueprints/BP_ThirdPersonCharacter.BP_ThirdPersonCharacter_C"))
          (for _array_element_2 _outactors_2
            (`self.K2_SetActorLocation` _array_element_2 (`/Game/Blueprints/BP_ThirdPersonCharacter.StartPosition` _array_element_2) false true))
          (`KismetSystemLibrary.Delay` 5.0)
          (goto _label :!via `Reset`))))))

(fn `UserConstructionScript`)